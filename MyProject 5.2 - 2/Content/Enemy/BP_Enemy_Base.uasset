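; Base enemy Blueprint that chases the player and plays montage-driven special and default attacks.
; Pawn sensing flags the player as seen and enables attacking; nothing in this graph starts the chase.
; ChasePlayer checks a game-time cooldown as each move begins, then on arrival special-attacks if allowed, waits and loops.
; Both attacks call their end events when montages complete or are interrupted; DefaultAttack is not invoked here.
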(event `self.PawnSensing.OnSeePawn`
  (params (Pawn :type "Pawn Object Reference"))
  ;[0.05127 0.05127 0.05127] On See Pawn
  (set `self.CanAttack` true)
  (set `self.HasSeenPlayer` true))

(event `ChasePlayer`
  ;[0.05127 0.05127 0.05127] Chase Player
  (`|AIMoveTo` self (0.0 0.0 0.0) (`GameplayStatics.GetPlayerCharacter` 0) 600.0
    (:`then`
      (`/Engine/EditorBlueprintResources/StandardMacros.CompareFloat` (`self.AttackCooldown`) (`KismetSystemLibrary.GetGameTimeInSeconds`)
        (:`>`
          (set `self.CanAttack` false :!label _label))
        (:`==`
          (goto _label))
        (:`<`
          (set `self.CanAttack` true))))
    (:`OnSuccess`
      (if (`self.CanAttack`)
        (`self.SpecialAttack`)
        (set `self.AttackCooldown` (+ (`KismetSystemLibrary.GetGameTimeInSeconds`) (`self.AttackingCooldown`)))
        (`KismetSystemLibrary.Delay` 4.0))
      (`self.ChasePlayer`))))

(event `SpecialAttack`
  ;[0.05127 0.05127 0.05127] Special Attack
  (`|PlayMontage` (`self.Mesh`) "/Game/Animations/Jump_Attack_Montage.Jump_Attack_Montage"
    (:`OnCompleted`
      _)
    (:`OnInterrupted`
      _))
  (`self.OnSpecialAttackEnd`))

(event `DefaultAttack`
  ;[0.05127 0.05127 0.05127] Default Attack
  (`|PlayMontage` (`self.Mesh`) "/Game/Animations/Standing_Attack_Montage.Standing_Attack_Montage"
    (:`OnCompleted`
      _)
    (:`OnInterrupted`
      _))
  (`self.OnDefaultAttackEnd`))

(fn `UserConstructionScript`)