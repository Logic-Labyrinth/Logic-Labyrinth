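; Base enemy Blueprint that provides player detection, two attacks and health helpers.
; PawnSensing sets the can-attack and seen-player flags whenever it sees a pawn, without filtering which pawn.
; Default and special attack events play standing and jump montages on the mesh, then fire their end dispatchers on completion or interruption.
; GetHealth returns enemy health, while UpdateHealth only returns an adjusted sum without storing it.
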(event `self.PawnSensing.OnSeePawn`
  (params (Pawn :type "Pawn Object Reference"))
  ;[0.05127 0.05127 0.05127] On See Pawn
  (set `self.CanAttack` true)
  (set `self.HasSeenPlayer` true))

(event `SpecialAttack`
  ;[0.05127 0.05127 0.05127] Special Attack
  (`|PlayMontage` (`self.Mesh`) "/Game/Animations/Jump_Attack_Montage.Jump_Attack_Montage"
    (:`OnCompleted`
      _)
    (:`OnInterrupted`
      _))
  (`self.OnSpecialAttackEnd`))

(event `DefaultAttack`
  ;[0.05127 0.05127 0.05127] Default Attack
  (`|PlayMontage` (`self.Mesh`) "/Game/Animations/Standing_Attack_Montage.Standing_Attack_Montage"
    (:`OnCompleted`
      _)
    (:`OnInterrupted`
      _))
  (`self.OnDefaultAttackEnd`))

(fn `GetHealth`
  (returns (EnemyHealth :type "Float (double-precision)"))
  (return (`self.EnemyHealth`)))

(fn `UpdateHealth`
  (params (EnemyHealth :type "Float (double-precision)") (HealthAdjustment :type "Float (double-precision)"))
  (returns (NewEnemyHealth :type "Float (double-precision)"))
  (return (+ EnemyHealth HealthAdjustment)))

(fn `UserConstructionScript`)